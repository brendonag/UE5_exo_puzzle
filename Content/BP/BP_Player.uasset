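; Player Blueprint that owns the gameplay HUD and pause menu widgets and handles their input.
; On BeginPlay it creates both widgets, hides the menu and passes it a reference to the HUD.
; The A key triggers the HUD's count-up event.
; P or Gamepad Special Right flips the HUD's Pause flag, swapping widget visibility, mouse cursor and click events, and focusing the menu without calling SetGamePaused.
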(event `self.ReceiveBeginPlay`
  (bind _hud_player (`self.HUD Player`))
  (bind _returnvalue (`|CreateWidget` "/Game/menu/HUD_Player2.HUD_Player2_C"))
  (set `/Game/menu/HUD_Player2.Pause` false _returnvalue)
  (set `self.HUD Player` _returnvalue)
  (bind _returnvalue_2 (`|CreateWidget` "/Game/menu/HUD_MenuPause.HUD_MenuPause_C"))
  (bind _output_get (set `self.HUD Pause` _returnvalue_2))
  (`Widget.SetVisibility` _output_get "Hidden")
  (bind _ashud_menu_pause (cast `/Game/menu/HUD_MenuPause` _output_get))
  (set `/Game/menu/HUD_MenuPause.HUD_player` _hud_player _ashud_menu_pause)
  (`UserWidget.AddToViewport` _hud_player 0)
  (`UserWidget.AddToViewport` (`self.HUD Pause`) 0))

(event `Key|A`
  (params (Key :type "Key Structure"))
  (:`Pressed`
    (`KismetSystemLibrary.PrintText` "A")
    (bind _ashud_player_2 (cast `/Game/menu/HUD_Player2` (`self.HUD Player`)))
    (`/Game/menu/HUD_Player2.UpCountEvent` _ashud_player_2)))

(event `Key|P`
  (params (Key :type "Key Structure"))
  (bind _returnvalue (`GameplayStatics.GetPlayerController` 0))
  (bind _hud_pause (`self.HUD Pause`))
  (:`Pressed`
    (`KismetSystemLibrary.PrintText` "P")
    (bind _ashud_player_2 (cast `/Game/menu/HUD_Player2` (`self.HUD Player`) :!label _label))
    (if (`/Game/menu/HUD_Player2.Pause` _ashud_player_2)
      (set `/Game/menu/HUD_Player2.Pause` false _ashud_player_2)
      (`Widget.SetVisibility` _ashud_player_2 "Visible")
      (`Widget.SetVisibility` _hud_pause "Hidden")
      (set `PlayerController.bShowMouseCursor` false _returnvalue)
      (set `PlayerController.bEnableClickEvents` false _returnvalue)
      (else
        (set `/Game/menu/HUD_Player2.Pause` true _ashud_player_2)
        (`Widget.SetVisibility` _ashud_player_2 "Hidden")
        (`Widget.SetVisibility` _hud_pause "Visible")
        (set `PlayerController.bShowMouseCursor` true _returnvalue)
        (set `PlayerController.bEnableClickEvents` true _returnvalue)
        (bind _ashud_menu_pause (cast `/Game/menu/HUD_MenuPause` _hud_pause))
        (`/Game/menu/HUD_MenuPause.Focus` _ashud_menu_pause)))))

(event `Key|Gamepad_Special_Right`
  (params (Key :type "Key Structure"))
  (:`Pressed`
    (goto _label)))

(fn `UserConstructionScript`)