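; Grid generator actor that builds a puzzle board of BP_Cell actors textured with a downloaded image.
; On BeginPlay it spawns cells using the grid size from GI_GridParam, leaving the (0,0) slot empty.
; It then downloads the game instance's image URL and gives each cell a dynamic M_Cell material with that texture.
; Each tile's offset derives from array index and GridSizeX, so the mapping assumes a square grid.
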(event `self.ReceiveBeginPlay`
  (bind _asgi_grid_param (cast `/Game/Blueprints/GI_GridParam` (`GameplayStatics.GetGameInstance`)))
  (for _index (range (`/Game/Blueprints/GI_GridParam.Grid Size X` _asgi_grid_param))
    (for _index_2 (range (`/Game/Blueprints/GI_GridParam.Grid Size Y` _asgi_grid_param))
      (if (not (and (== _index_2 0) (== _index 0)))
        (bind _returnvalue (`|SpawnActorFromClass` "/Game/Blueprints/BP_Cell.BP_Cell_C" (`KismetMathLibrary.MakeTransform` (`KismetMathLibrary.MakeVector` (* (`KismetMathLibrary.Conv_IntToDouble` _index) (`self.GridCellOffset`)) (* (`KismetMathLibrary.Conv_IntToDouble` _index_2) (`self.GridCellOffset`)))) "Undefined" "OverrideRootScale" null null))
        (`KismetArrayLibrary.Array_Add` (`self.GridCells`) _returnvalue))))
  (`self.UpdatePuzzleImage` (`/Game/Blueprints/GI_GridParam.ImageURL` _asgi_grid_param)))

(event `UpdatePuzzleImage`
  (params (URL :type String))
  (bind _texture (`AsyncTaskDownloadImage.DownloadImage` URL)
    (:`OnSuccess`
      (for (_array_element _array_index) (`self.GridCells`)
        (bind _returnvalue (`KismetMaterialLibrary.CreateDynamicMaterialInstance` "/Game/Mats/M_Cell.M_Cell"))
        (`MaterialInstanceDynamic.SetTextureParameterValue` _returnvalue "PuzzleTexture" _texture)
        (bind _asgi_grid_param (cast `/Game/Blueprints/GI_GridParam` (`GameplayStatics.GetGameInstance`)))
        (bind _returnvalue_2 (+ _array_index 1))
        (bind _grid_size_x (`/Game/Blueprints/GI_GridParam.Grid Size X` _asgi_grid_param))
        (`MaterialInstanceDynamic.SetVectorParameterValue` _returnvalue "TextureOffset2d" (make `LinearColor` (`KismetMathLibrary.Conv_IntToDouble` (/ _returnvalue_2 _grid_size_x)) (`KismetMathLibrary.Conv_IntToDouble` (mod _returnvalue_2 _grid_size_x)) (`KismetMathLibrary.Conv_IntToDouble` (* _grid_size_x (`/Game/Blueprints/GI_GridParam.Grid Size Y` _asgi_grid_param))) 1.0))
        (`PrimitiveComponent.SetMaterial` (`/Game/Blueprints/BP_Cell.Cube` _array_element) 0 _returnvalue)))))

(fn `UserConstructionScript`)