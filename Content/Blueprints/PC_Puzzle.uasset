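; Player controller for a board puzzle that relays directional key presses to the controlled board player.
; It enables input on BeginPlay and binds the Up, Right, Down and Left keys directly.
; Each press casts the controlled pawn to BP_BoardPlayer and calls GetInput with that direction's enum value, leaving the response to the pawn.
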(event `self.ReceiveBeginPlay`
  (`self.EnableInput` null))

(event `Key|Up`
  (params (Key :type "Key Structure"))
  (:`Pressed`
    (bind _asbp_board_player (cast `/Game/Blueprints/BP_BoardPlayer` (`self.K2_GetPawn`)))
    (`/Game/Blueprints/BP_BoardPlayer.GetInput` _asbp_board_player "NewEnumerator2")))

(event `Key|Right`
  (params (Key :type "Key Structure"))
  (:`Pressed`
    (bind _asbp_board_player (cast `/Game/Blueprints/BP_BoardPlayer` (`self.K2_GetPawn`)))
    (`/Game/Blueprints/BP_BoardPlayer.GetInput` _asbp_board_player "NewEnumerator1")))

(event `Key|Down`
  (params (Key :type "Key Structure"))
  (:`Pressed`
    (bind _asbp_board_player (cast `/Game/Blueprints/BP_BoardPlayer` (`self.K2_GetPawn`)))
    (`/Game/Blueprints/BP_BoardPlayer.GetInput` _asbp_board_player "NewEnumerator0")))

(event `Key|Left`
  (params (Key :type "Key Structure"))
  (:`Pressed`
    (bind _asbp_board_player (cast `/Game/Blueprints/BP_BoardPlayer` (`self.K2_GetPawn`)))
    (`/Game/Blueprints/BP_BoardPlayer.GetInput` _asbp_board_player "NewEnumerator3")))

(fn `UserConstructionScript`)