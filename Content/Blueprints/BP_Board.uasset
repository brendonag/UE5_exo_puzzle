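; BP_Board builds a grid of BP_Tile actors to form the game board.
; On BeginPlay, if ListTiles is empty, nested loops over Lines and Columns spawn tiles spaced by Offset along world X and Y, independent of the board's own location.
; Each tile is stored in ListTiles and receives the board's Offset and SpeedMove values.
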(event `self.ReceiveBeginPlay`
  (bind _offset (`self.Offset`))
  (if (not (> (`KismetArrayLibrary.Array_Length` (`self.ListTiles`)) 0))
    (for _index (range (`self.Lines`))
      (for _index_2 (range (`self.Columns`))
        (bind _returnvalue (`|SpawnActorFromClass` "/Game/Blueprints/BP_Tile.BP_Tile_C" (`KismetMathLibrary.MakeTransform` (`KismetMathLibrary.MakeVector` (* (`KismetMathLibrary.Conv_IntToDouble` _index) _offset) (* _offset _index_2))) "Undefined" "OverrideRootScale" null null))
        (`KismetArrayLibrary.Array_Add` (`self.ListTiles`) _returnvalue)
        (set `/Game/Blueprints/BP_Tile.f_offset` (`self.Offset`) _returnvalue)
        (`/Game/Blueprints/BP_Tile.SetSpeedMove` _returnvalue (`self.SpeedMove`))))))

(fn `UserConstructionScript`)