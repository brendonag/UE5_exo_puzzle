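; Board player that steps tile to tile and carries a spring-arm camera with pan, rotate, zoom and focus controls.
; Directional input fills a two-slot queue that OnAction drains on a short delay.
; Each step line-traces for a neighbouring BP_Tile, moves the player onto it, triggers the tile's movement and plays a random-pitch pop.
; Timelines blend the camera between angled and top-down views, with rotation locked in top view.
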(event `Right / Left`
  (params (`Axis Value` :type "Float (double-precision)"))
  (bind _springarm (`self.SpringArm`))
  (bind (_returnvalue_x _returnvalue_y _returnvalue_z) (`KismetMathLibrary.BreakVector` (`SceneComponent.K2_GetComponentLocation` _springarm)))
  ;[0 0 0] CAMERA
  ;;[0.3916 1 0.3005] POSITION
  (`SceneComponent.K2_SetWorldLocation` _springarm (`KismetMathLibrary.MakeVector` (+ (* `Axis Value` 20.0) _returnvalue_x) (+ _returnvalue_y (* (stale `Forward / Backward` `Axis Value`) 20.0)) _returnvalue_z) false false :!label _label))

(event `Pitch`
  (params (`Axis Value` :type "Float (double-precision)"))
  (bind _springarm (`self.SpringArm`))
  (bind (_returnvalue_roll _returnvalue_pitch _returnvalue_yaw) (`KismetMathLibrary.BreakRotator` (`SceneComponent.K2_GetComponentRotation` _springarm)))
  ;[0 0 0] CAMERA
  ;;[1 0.8469 0.1912] ROTATION
  (if (not (`self.inTopView`))
    (`SceneComponent.K2_SetWorldRotation` _springarm (`KismetMathLibrary.MakeRotator` _returnvalue_roll (`KismetMathLibrary.FClamp` (+ `Axis Value` _returnvalue_pitch) -80.0 0.0) (`KismetMathLibrary.FClamp` (+ _returnvalue_yaw (stale `Yaw` `Axis Value`)) -120.0 -60.0)) false false :!label _label_2)))

(event `GetInput`
  (params (NewParam :type "/Game/Blueprints/E_Directions Enum" :default "NewEnumerator0"))
  (bind _oppositedir (`self.oppositeDir`))
  ;[0 0 0] ACTION
  ;;[0.4897 0.8608 1] PLAYER TILE
  (if (< (`KismetArrayLibrary.Array_Length` (`self.oppositeDir`)) 2)
    (switch `/Game/Blueprints/E_Directions` NewParam
      (:`NewEnumerator0`
        (`KismetArrayLibrary.Array_Add` _oppositedir "NewEnumerator0"))
      (:`NewEnumerator1`
        (`KismetArrayLibrary.Array_Add` _oppositedir "NewEnumerator1"))
      (:`NewEnumerator2`
        (`KismetArrayLibrary.Array_Add` _oppositedir "NewEnumerator2"))
      (:`NewEnumerator3`
        (`KismetArrayLibrary.Array_Add` _oppositedir "NewEnumerator3")))
    (`self.ActivateMouvement`)))

(event `Yaw`
  (params (`Axis Value` :type "Float (double-precision)"))
  ;[0 0 0] CAMERA
  ;;[1 0.8469 0.1912] ROTATION
  (if (not (`self.inTopView`))
    (goto _label_2)))

(event `ActivateMouvement`
  (bind _returnvalue (`self.K2_GetActorLocation`))
  (bind _pop (`self.Pop`))
  ;[0 0 0] ACTION
  ;;[0.4897 0.8608 1] PLAYER TILE
  (`|ExecutionSequence`
    (:`then_0`
      (if (`self.canTakeInput`)
        (set `self.canTakeInput` false)
        (bind _output_get (set `self.SaveEnum` (`|GetArrayItem` (`self.oppositeDir`))))
        (switch `/Game/Blueprints/E_Directions` _output_get
          (:`NewEnumerator0`
            (set `self.v_dir` (0.0 1.0 0.0)))
          (:`NewEnumerator1`
            (set `self.v_dir` (1.0 0.0 0.0)))
          (:`NewEnumerator2`
            (set `self.v_dir` (0.0 -1.0 0.0)))
          (:`NewEnumerator3`
            (set `self.v_dir` (-1.0 0.0 0.0))))
        (`KismetArrayLibrary.Array_Remove` (`self.oppositeDir`))
        (bind (_outhit _returnvalue_2) (`KismetSystemLibrary.LineTraceSingle` _returnvalue (+ _returnvalue (* (`self.v_dir`) (`self.f_sizeTile`))) "TraceTypeQuery1"))
        (if _returnvalue_2
          (bind _asbp_tile (cast `/Game/Blueprints/BP_Tile` (`.HitActor` (`GameplayStatics.BreakHitResult` _outhit)))
            (:`then`
              (`self.K2_SetActorLocation` (`self.K2_GetActorLocation` _asbp_tile))
              (`/Game/Blueprints/BP_Tile.LaunchMovement` _asbp_tile (`self.SaveEnum`))
              (set `AudioComponent.PitchMultiplier` (`KismetMathLibrary.RandomFloatInRange` 0.5 1.5) _pop)
              (`AudioComponent.Play` _pop 0.0))
            (:`CastFailed`
              (`KismetSystemLibrary.PrintString` "Not a tile")))
          (else
            (`KismetSystemLibrary.PrintString` "No hit detected")))))
    (:`then_1`
      (`KismetSystemLibrary.Delay` 0.2)
      (set `self.canTakeInput` true)
      (if (> (`KismetArrayLibrary.Array_Length` (`self.oppositeDir`)) 0)
        (`self.ActivateMouvement`)))))

(event `Forward / Backward`
  (params (`Axis Value` :type "Float (double-precision)"))
  ;[0 0 0] CAMERA
  ;;[0.3916 1 0.3005] POSITION
  (goto _label))

(event `Zoom`
  (params (`Wheel Value` :type "Float (double-precision)"))
  (bind _springarm (`self.SpringArm`))
  ;[0 0 0] CAMERA
  ;;[1 0.2051 0.5029] ZOOM
  (set `SpringArmComponent.TargetArmLength` (`KismetMathLibrary.FClamp` (+ (* `Wheel Value` 50.0) (`SpringArmComponent.TargetArmLength` _springarm)) 100.0 10000.0) _springarm))

(event `TopView`
  (bind _springarm (`self.SpringArm`))
  (bind _springarm_2 (`self.SpringArm`))
  ;[0 0 0] CAMERA
  ;;[0.6376 0.6724 1] POINT OF VIEW
  (if (not (`self.animChangeView`))
    (`/Engine/EditorBlueprintResources/StandardMacros.FlipFlop`
      (:`A`
        (set `self.animChangeView` true)
        (`|ExecutionSequence`
          (:`then_0`
            (set `self.inTopView` true))
          (:`then_1`
            (bind (_direction _lerpthis) (`Timeline|Timeline_0` :!via `PlayFromStart`)
              (:`Update`
                (`SceneComponent.K2_SetWorldRotation` _springarm_2 (`KismetMathLibrary.RLerp` (`SceneComponent.K2_GetComponentRotation` _springarm_2) (`KismetMathLibrary.MakeRotator` 0.0 -90.0 -90.0) _lerpthis true) false false))
              (:`Finished`
                (set `self.animChangeView` false))))))
      (:`B`
        (set `self.animChangeView` true)
        (bind (_direction_2 _lerpthis_2) (`Timeline|Timeline_1` :!via `PlayFromStart`)
          (:`Update`
            (`SceneComponent.K2_SetWorldRotation` _springarm (`KismetMathLibrary.RLerp` (`SceneComponent.K2_GetComponentRotation` _springarm) (`KismetMathLibrary.MakeRotator` 0.0 -50.0 -90.0) _lerpthis_2 true) false false))
          (:`Finished`
            (set `self.animChangeView` false)
            (set `self.inTopView` false)))))))

(event `Focus`
  (bind _springarm (`self.SpringArm`))
  ;[0 0 0] CAMERA
  ;;[1 1 1] FOCUS
  (if (`self.inTopView`)
    (`SceneComponent.K2_SetWorldLocationAndRotation` _springarm (0.0 0.0 0.0) (struct :`Pitch` -90.0 :`Yaw` -90.0) false true)
    (set `SpringArmComponent.TargetArmLength` 500.0 _springarm)
    (else
      (`SceneComponent.K2_SetWorldLocationAndRotation` _springarm (0.0 0.0 0.0) (struct :`Pitch` -50.0 :`Yaw` -90.0) false true)
      (set `SpringArmComponent.TargetArmLength` 500.0 _springarm))))

(fn `UserConstructionScript`)