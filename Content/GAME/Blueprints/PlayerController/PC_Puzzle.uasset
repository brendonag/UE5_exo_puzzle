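; Player controller for the puzzle board that turns player input into commands on the controlled BP_BoardPlayer pawn.
; Axis inputs drive camera movement, pitch, yaw and zoom, while action inputs trigger top view, focus and pause.
; The four directional actions each pass an enum value to the pawn's GetInput.
; Every handler casts the controlled pawn and forwards the call, so the controller holds no game logic itself.
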(event `InputAxis|Move Forward / Backward`
  (params (AxisValue :type "Float (single-precision)"))
  ;[0 0 0] CAMERA
  ;;[0.3916 1 0.3005] POSITION
  (bind _asbp_board_player (cast `/Game/GAME/Blueprints/Pawn/BP_BoardPlayer` (`self.K2_GetPawn`)))
  (`/Game/GAME/Blueprints/Pawn/BP_BoardPlayer.Forward / Backward` _asbp_board_player AxisValue))

(event `InputAxis|Pitch`
  (params (AxisValue :type "Float (single-precision)"))
  ;[0 0 0] CAMERA
  ;;[1 0.8469 0.1912] ROTATION
  (bind _asbp_board_player (cast `/Game/GAME/Blueprints/Pawn/BP_BoardPlayer` (`self.K2_GetPawn`)))
  (`/Game/GAME/Blueprints/Pawn/BP_BoardPlayer.Pitch` _asbp_board_player AxisValue))

(event `InputAxis|Move Right / Left`
  (params (AxisValue :type "Float (single-precision)"))
  ;[0 0 0] CAMERA
  ;;[0.3916 1 0.3005] POSITION
  (bind _asbp_board_player (cast `/Game/GAME/Blueprints/Pawn/BP_BoardPlayer` (`self.K2_GetPawn`)))
  (`/Game/GAME/Blueprints/Pawn/BP_BoardPlayer.Right / Left` _asbp_board_player AxisValue))

(event `InputAxis|Yaw`
  (params (AxisValue :type "Float (single-precision)"))
  ;[0 0 0] CAMERA
  ;;[1 0.8469 0.1912] ROTATION
  (bind _asbp_board_player (cast `/Game/GAME/Blueprints/Pawn/BP_BoardPlayer` (`self.K2_GetPawn`)))
  (`/Game/GAME/Blueprints/Pawn/BP_BoardPlayer.Yaw` _asbp_board_player AxisValue))

(event `InputAction|TopView`
  (params (Key :type "Key Structure"))
  ;[0 0 0] CAMERA
  ;;[0.6376 0.6724 1] POINT OF VIEW
  (:`Pressed`
    (bind _asbp_board_player (cast `/Game/GAME/Blueprints/Pawn/BP_BoardPlayer` (`self.K2_GetPawn`)))
    (`/Game/GAME/Blueprints/Pawn/BP_BoardPlayer.TopView` _asbp_board_player)))

(event `InputAxis|Zoom`
  (params (AxisValue :type "Float (single-precision)"))
  ;[0 0 0] CAMERA
  ;;[1 0.2051 0.5029] ZOOM
  (bind _asbp_board_player (cast `/Game/GAME/Blueprints/Pawn/BP_BoardPlayer` (`self.K2_GetPawn`)))
  (`/Game/GAME/Blueprints/Pawn/BP_BoardPlayer.Zoom` _asbp_board_player AxisValue))

(event `InputAction|Focus`
  (params (Key :type "Key Structure"))
  ;[1 1 1] FOCUS ON GAME
  (:`Pressed`
    (bind _asbp_board_player (cast `/Game/GAME/Blueprints/Pawn/BP_BoardPlayer` (`self.K2_GetPawn`)))
    (`/Game/GAME/Blueprints/Pawn/BP_BoardPlayer.Focus` _asbp_board_player)))

(event `InputAction|UP`
  (params (Key :type "Key Structure"))
  ;[0 0 0] ACTION
  ;;[0.2918 0.855 1] OnAction
  (:`Pressed`
    (bind _asbp_board_player (cast `/Game/GAME/Blueprints/Pawn/BP_BoardPlayer` (`self.K2_GetPawn`)))
    (`/Game/GAME/Blueprints/Pawn/BP_BoardPlayer.GetInput` _asbp_board_player "NewEnumerator2")))

(event `InputAction|RIGHT`
  (params (Key :type "Key Structure"))
  ;[0 0 0] ACTION
  ;;[0.2918 0.855 1] OnAction
  (:`Pressed`
    (bind _asbp_board_player (cast `/Game/GAME/Blueprints/Pawn/BP_BoardPlayer` (`self.K2_GetPawn`)))
    (`/Game/GAME/Blueprints/Pawn/BP_BoardPlayer.GetInput` _asbp_board_player "NewEnumerator1")))

(event `InputAction|PAUSE`
  (params (Key :type "Key Structure"))
  ;[1 1 1] PAUSE
  (:`Pressed`
    (bind _asbp_board_player (cast `/Game/GAME/Blueprints/Pawn/BP_BoardPlayer` (`self.K2_GetPawn`)))
    (`/Game/GAME/Blueprints/Pawn/BP_BoardPlayer.Pause` _asbp_board_player)))

(event `InputAction|Down`
  (params (Key :type "Key Structure"))
  ;[0 0 0] ACTION
  ;;[0.2918 0.855 1] OnAction
  (:`Pressed`
    (bind _asbp_board_player (cast `/Game/GAME/Blueprints/Pawn/BP_BoardPlayer` (`self.K2_GetPawn`)))
    (`/Game/GAME/Blueprints/Pawn/BP_BoardPlayer.GetInput` _asbp_board_player "NewEnumerator0")))

(event `InputAction|LEFT`
  (params (Key :type "Key Structure"))
  ;[0 0 0] ACTION
  ;;[0.2918 0.855 1] OnAction
  (:`Pressed`
    (bind _asbp_board_player (cast `/Game/GAME/Blueprints/Pawn/BP_BoardPlayer` (`self.K2_GetPawn`)))
    (`/Game/GAME/Blueprints/Pawn/BP_BoardPlayer.GetInput` _asbp_board_player "NewEnumerator3")))

(fn `UserConstructionScript`)