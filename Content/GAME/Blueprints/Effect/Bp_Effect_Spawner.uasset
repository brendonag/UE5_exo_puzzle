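; Effect spawner Blueprint exposing events that trigger particles, sounds and camera shakes.
; SpawnParticles spawns an emitter at a location and applies the given lifespan to that component's owner.
; SpawnAudioEffect plays a non-spatial 2D sound, repeating after its duration while Loop is set, then destroys a placeholder actor spawned at Position.
; CameraShake adds a shake source component to the supplied camera and starts the requested shake at a given scale.
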(event `Spawn Particles`
  (params (Particle_Asset :type "ParticleSystem Object Reference") (LifeTime :type "Float (double-precision)") (Position :type "Transform Structure"))
  (bind _returnvalue (`GameplayStatics.SpawnEmitterAtLocation` Particle_Asset Position_Location))
  (`self.SetLifeSpan` (`ActorComponent.GetOwner` _returnvalue) LifeTime))

(event `Spawn Audio Effect`
  (params (Loop :type Boolean) (`Sound ` :type "SoundBase Object Reference") (Position :type "Transform Structure"))
  (bind _returnvalue (`|SpawnActorFromClass` "/Script/Engine.Actor" Position "Undefined" "OverrideRootScale" null null))
  (bind _returnvalue_2 (`GameplayStatics.CreateSound2D` `Sound ` 1.0 1.0 0.0 null))
  (bind _sound (`AudioComponent.Sound` _returnvalue_2))
  (`GameplayStatics.PlaySound2D` _sound 1.0 1.0 0.0 null null)
  (bind _duration (`SoundBase.Duration` _sound))
  (`KismetSystemLibrary.Delay` _duration)
  (while Loop
    (`GameplayStatics.PlaySound2D` _sound 1.0 1.0 0.0 null null)
    (`KismetSystemLibrary.Delay` _duration))
  (`self.K2_DestroyActor` _returnvalue))

(event `Camera Shake`
  (params (Camera :type "CameraActor Object Reference") (InCameraShake :type "CameraShakeBase Class Reference") (Scale :type "Float (single-precision)"))
  (bind _returnvalue (`AddComponent|NODE_AddCameraShakeSourceComponent-0` :`self` Camera))
  (`CameraShakeSourceComponent.StartCameraShake` :`self` _returnvalue :`InCameraShake` InCameraShake :`Scale` Scale))

(fn `UserConstructionScript`)