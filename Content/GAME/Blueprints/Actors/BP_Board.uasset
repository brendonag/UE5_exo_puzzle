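; BP_Board builds and shuffles a sliding picture puzzle.
; On BeginPlay it spawns a BP_Tile grid sized by GI_GridParam, then downloads the image and maps a slice onto each tile through M_Cell dynamic materials.
; After download, it replaces a random tile with a possessed BP_BoardPlayer as the gap.
; A looping timer shuffles by feeding that pawn random direction inputs, with the GameInstance IsShuffling flag set until done.
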(event `self.ReceiveBeginPlay`
  (bind _offset (`self.Offset`))
  (bind _asgi_grid_param (cast `/Game/GAME/Blueprints/GameInstance/GI_GridParam` (`GameplayStatics.GetGameInstance`)))
  (if (not (> (`KismetArrayLibrary.Array_Length` (`self.ListTiles`)) 0))
    (for _index (range (`/Game/GAME/Blueprints/GameInstance/GI_GridParam.Grid Size X` _asgi_grid_param))
      (for _index_2 (range (`/Game/GAME/Blueprints/GameInstance/GI_GridParam.Grid Size Y` _asgi_grid_param))
        (bind _returnvalue (`|SpawnActorFromClass` "/Game/GAME/Blueprints/Actors/BP_Tile.BP_Tile_C" (`KismetMathLibrary.MakeTransform` (`KismetMathLibrary.MakeVector` (* (`KismetMathLibrary.Conv_IntToDouble` _index) _offset) (* _offset _index_2))) "Undefined" "OverrideRootScale" null null))
        (`KismetArrayLibrary.Array_Add` (`self.ListTiles`) _returnvalue)
        (set `/Game/GAME/Blueprints/Actors/BP_Tile.f_offset` (`self.Offset`) _returnvalue)
        (`/Game/GAME/Blueprints/Actors/BP_Tile.SetSpeedMove` _returnvalue (`self.SpeedMove`))))
    (`self.UpdatePuzzleImage` (`/Game/GAME/Blueprints/GameInstance/GI_GridParam.ImageURL` _asgi_grid_param))))

(event `SpawnPlayer`
  (bind _result (`/Engine/EditorBlueprintResources/StandardMacros.DecrementInt` (`KismetArrayLibrary.Array_Length` (`self.listTiles`)))
    (:`  `
      (bind _output_get (set `self.random` (`KismetMathLibrary.RandomInteger` _result)))
      (bind _output (`|GetArrayItem` (`self.listTiles`) _output_get))
      (bind _returnvalue (`|SpawnActorFromClass` "/Game/GAME/Blueprints/Pawn/BP_BoardPlayer.BP_BoardPlayer_C" (`KismetMathLibrary.MakeTransform` (`self.K2_GetActorLocation` _output)) "AlwaysSpawn" "OverrideRootScale" null null))
      (`self.K2_DestroyActor` _output)
      (`Controller.Possess` (`GameplayStatics.GetPlayerController` 0) _returnvalue)
      (`self.RandomizeMap`))))

(event `UpdatePuzzleImage`
  (params (URL :type String))
  (bind _texture (`AsyncTaskDownloadImage.DownloadImage` URL)
    (:`OnSuccess`
      (for (_array_element _array_index) (`self.listTiles`)
        (bind _returnvalue (`KismetMaterialLibrary.CreateDynamicMaterialInstance` "/Game/GAME/Mats/M_Cell.M_Cell"))
        (`MaterialInstanceDynamic.SetTextureParameterValue` _returnvalue "PuzzleTexture" _texture)
        (bind _asgi_grid_param (cast `/Game/GAME/Blueprints/GameInstance/GI_GridParam` (`GameplayStatics.GetGameInstance`)))
        (bind _returnvalue_2 (+ _array_index 0))
        (bind _grid_size_y (`/Game/GAME/Blueprints/GameInstance/GI_GridParam.Grid Size Y` _asgi_grid_param))
        (`MaterialInstanceDynamic.SetVectorParameterValue` _returnvalue "TextureOffset2d" (make `LinearColor` (`KismetMathLibrary.Conv_IntToDouble` (/ _returnvalue_2 _grid_size_y)) (`KismetMathLibrary.Conv_IntToDouble` (mod _returnvalue_2 _grid_size_y)) (`KismetMathLibrary.Conv_IntToDouble` _grid_size_y) 1.0))
        (`PrimitiveComponent.SetMaterial` (`/Game/GAME/Blueprints/Actors/BP_Tile.Cube` _array_element) 0 _returnvalue))
      (`self.SpawnPlayer`))))

(event `RandomizeMap`
  (bind _asgi_grid_param (cast `/Game/GAME/Blueprints/GameInstance/GI_GridParam` (`GameplayStatics.GetGameInstance`)))
  (set `/Game/GAME/Blueprints/GameInstance/GI_GridParam.IsShuffling` true _asgi_grid_param)
  (bind _asbp_board_player (cast `/Game/GAME/Blueprints/Pawn/BP_BoardPlayer` (`GameplayStatics.GetPlayerPawn` 0)))
  (bind _returnvalue (`KismetSystemLibrary.K2_SetTimerDelegate` (delegate `RdmInput`) 0.2 true)))

(event `RdmInput`
  (if (< (`self.ShuffleCounter`) (`self.ShuffleNumber`))
    (switch `int` (`KismetMathLibrary.RandomInteger` 4)
      (:`0`
        (`/Game/GAME/Blueprints/Pawn/BP_BoardPlayer.GetInput` (stale `RandomizeMap` _asbp_board_player) "NewEnumerator0"))
      (:`1`
        (`/Game/GAME/Blueprints/Pawn/BP_BoardPlayer.GetInput` (stale `RandomizeMap` _asbp_board_player) "NewEnumerator1"))
      (:`2`
        (`/Game/GAME/Blueprints/Pawn/BP_BoardPlayer.GetInput` (stale `RandomizeMap` _asbp_board_player) "NewEnumerator2"))
      (:`3`
        (`/Game/GAME/Blueprints/Pawn/BP_BoardPlayer.GetInput` (stale `RandomizeMap` _asbp_board_player) "NewEnumerator3")))
    (`/Engine/EditorBlueprintResources/StandardMacros.IncrementInt` (`self.ShuffleCounter`))
    (else
      (`KismetSystemLibrary.K2_ClearAndInvalidateTimerHandle` (stale `RandomizeMap` _returnvalue))
      (bind _asgi_grid_param (cast `/Game/GAME/Blueprints/GameInstance/GI_GridParam` (`GameplayStatics.GetGameInstance`)))
      (set `/Game/GAME/Blueprints/GameInstance/GI_GridParam.IsShuffling` false _asgi_grid_param))))

(fn `UserConstructionScript`)