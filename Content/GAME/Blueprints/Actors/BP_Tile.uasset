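; BP_Tile is a tile actor that slides one offset step in a given direction along world X or Y.
; LaunchMovement ignores calls while moving, stores the start location, derives the target from direction and FOffset, then lerps there on a timeline.
; SetSpeedMove changes the timeline play rate.
; A debug click handler moves the tile up and prints the offset, but its binding never runs.
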(event `self.ReceiveBeginPlay`)

(event `OnClicked_Event` :!signature `self.OnClicked`
  (params (TouchedActor :type "Actor Object Reference") (ButtonPressed :type "Key Structure" :default "None"))
  (`self.LaunchMovement` "NewEnumerator0")
  (`KismetSystemLibrary.PrintString` (`KismetStringLibrary.Conv_DoubleToString` (`self.f_offset`))))

(event `LaunchMovement`
  (params (Direction :type "/Game/GAME/Blueprints/Enums/E_Directions Enum" :default "NewEnumerator0"))
  (if (not (`self.b_isMoving`))
    (set `self.b_isMoving` true)
    (set `self.v_initialPos` (`self.K2_GetActorLocation`))
    (switch `/Game/GAME/Blueprints/Enums/E_Directions` Direction
      (:`NewEnumerator0`
        (`self.Set Target Location` (0.0 -1.0 0.0))
        (bind (_direction _newtrack_0) (`Timeline|Timeline_Mouvement` :!via `PlayFromStart` :!label _label)
          (:`Update`
            (`self.K2_SetActorLocation` (`KismetMathLibrary.VLerp` (`self.v_initialPos`) (`self.v_targetPos`) _newtrack_0)))
          (:`Finished`
            (set `self.b_isMoving` false))))
      (:`NewEnumerator1`
        (`self.Set Target Location` (-1.0 0.0 0.0))
        (goto _label :!via `PlayFromStart`))
      (:`NewEnumerator2`
        (`self.Set Target Location` (0.0 1.0 0.0))
        (goto _label :!via `PlayFromStart`))
      (:`NewEnumerator3`
        (`self.Set Target Location` (1.0 0.0 0.0))
        (goto _label :!via `PlayFromStart`)))))

(fn `Set Target Location`
  (params (v_dir :type "Vector Structure"))
  (set `self.v_targetPos` (+ (* v_dir (`self.f_offset`)) (`self.v_initialPos`))))

(fn `SetSpeedMove`
  (params (Speed :type "Float (double-precision)"))
  (`TimelineComponent.SetPlayRate` (`self.Timeline_Mouvement`) Speed))

(fn `UserConstructionScript`)