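; Player controller for the in-game camera that relays player input to the controlled P_CamInGame pawn.
; Movement, pitch and yaw axes and the TopView action each cast the controlled pawn and call its matching function, leaving the camera logic to the pawn.
; The Zoom axis event is present but has no logic.
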(event `InputAxis|Move Forward / Backward`
  (params (AxisValue :type "Float (single-precision)"))
  ;[0.3916 1 0.3005] POSITION
  (bind _asp_cam_in_game (cast `/Game/GAME/CamInGame/P_CamInGame` (`self.K2_GetPawn`)))
  (`/Game/GAME/CamInGame/P_CamInGame.Forward / Backward` _asp_cam_in_game AxisValue))

(event `InputAxis|Pitch`
  (params (AxisValue :type "Float (single-precision)"))
  ;[1 0.8469 0.1912] ROTATION
  (bind _asp_cam_in_game (cast `/Game/GAME/CamInGame/P_CamInGame` (`self.K2_GetPawn`)))
  (`/Game/GAME/CamInGame/P_CamInGame.Pitch` _asp_cam_in_game AxisValue))

(event `InputAxis|Yaw`
  (params (AxisValue :type "Float (single-precision)"))
  ;[1 0.8469 0.1912] ROTATION
  (bind _asp_cam_in_game (cast `/Game/GAME/CamInGame/P_CamInGame` (`self.K2_GetPawn`)))
  (`/Game/GAME/CamInGame/P_CamInGame.Yaw` _asp_cam_in_game AxisValue))

(event `InputAxis|Move Right / Left`
  (params (AxisValue :type "Float (single-precision)"))
  ;[0.3916 1 0.3005] POSITION
  (bind _asp_cam_in_game (cast `/Game/GAME/CamInGame/P_CamInGame` (`self.K2_GetPawn`)))
  (`/Game/GAME/CamInGame/P_CamInGame.Right / Left` _asp_cam_in_game AxisValue))

(event `InputAction|TopView`
  (params (Key :type "Key Structure"))
  (:`Pressed`
    (bind _asp_cam_in_game (cast `/Game/GAME/CamInGame/P_CamInGame` (`self.K2_GetPawn`)))
    (`/Game/GAME/CamInGame/P_CamInGame.TopView` _asp_cam_in_game)))

(event `InputAxis|Zoom`
  (params (AxisValue :type "Float (single-precision)")))

(fn `UserConstructionScript`)